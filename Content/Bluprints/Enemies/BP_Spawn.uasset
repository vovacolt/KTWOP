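; Enemy spawner actor that repeatedly spawns an enemy of a configurable class just above its root component.
; Tick feeds a Delay node, so the Delay variable sets the interval between spawns with no explicit timer or limit.
; Each spawn is cast to BP_TestEnemy to receive the spawner's Aim, a cast noted for later replacement by a base class.
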(event `self.ReceiveBeginPlay`)

(event `self.ReceiveTick`
  (params (DeltaSeconds :type "Float (single-precision)"))
  (`KismetSystemLibrary.Delay` (`self.Delay`))
  (bind _returnvalue (`|SpawnActorFromClass` (`self.EnemyType`) (`KismetMathLibrary.MakeTransform` (+ (`SceneComponent.K2_GetComponentLocation` (`self.DefaultSceneRoot`)) (`KismetMathLibrary.MakeVector` 0.0 0.0 50.0))) "Undefined" "OverrideRootScale" null null))
  ;[1 1 1] To base class later...
  (bind _asbp_test_enemy (cast `/Game/Bluprints/Enemies/BP_TestEnemy` _returnvalue))
  (set `/Game/Bluprints/Enemies/BP_TestEnemy.Aim` (`self.Aim`) _asbp_test_enemy))

(fn `UserConstructionScript`)